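; BP_ClickBox is a clickable box that cycles a single-digit number shown on its TextRender.
; Clicking ClickableBox counts up and the Bababooey event counts down, wrapping between 0 and 9.
; Both share one display update, also exposed as Refreshnumber, which shows zero as blank.
; Number starts at 1 on BeginPlay without refreshing the text, and getrowandcolumn only calls AddReturnResultsTerminal.
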(event OnClicked(ClickableBox)
  (params (TouchedComponent :type Primitive%20Component%20Object%20Reference) (ButtonPressed :type Key%20Structure :default "None"))
  (bind _textrender (Variables|Default|GetTextRender))
  (Math|Integer|IncrementInt (Variables|Default|GetNumber)
    (:%20%20
      (if (== (Variables|Default|GetNumber) 10)
        (Variables|Default|SetNumber 0))
      (if (== 0 (Variables|Default|GetNumber))
        (Rendering|Components|TextRender|SetText _textrender (Variables|Default|GetBlank))
        (else
          (Rendering|Components|TextRender|SetText _textrender (Utilities|Text|ToText(Integer) (Variables|Default|GetNumber))))))))

(event Custom|Refresh%20number
  (bind _textrender (Variables|Default|GetTextRender))
  (bind _number (Variables|Default|GetNumber))
  (if (== 0 _number)
    (Rendering|Components|TextRender|SetText _textrender (Variables|Default|GetBlank))
    (else
      (Rendering|Components|TextRender|SetText _textrender (Utilities|Text|ToText(Integer) _number)))))

(event Custom|Bababooey
  (bind _textrender (Variables|Default|GetTextRender))
  (Math|Integer|DecrementInt (Variables|Default|GetNumber)
    (:%20%20
      (if (== (Variables|Default|GetNumber) -1)
        (Variables|Default|SetNumber 9))
      (if (== 0 (Variables|Default|GetNumber))
        (Rendering|Components|TextRender|SetText _textrender (Variables|Default|GetBlank))
        (else
          (Rendering|Components|TextRender|SetText _textrender (Utilities|Text|ToText(Integer) (Variables|Default|GetNumber))))))))

(event Custom|get%20row%20and%20column
  (AddComponent|AddReturnResultsTerminal))

(event EventBeginPlay
  (Variables|Default|SetNumber 1))

(fn ConstructionScript)

(fn NewFunction)